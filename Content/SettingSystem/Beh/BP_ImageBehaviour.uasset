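; BP_ImageBehaviour is a setting-system behaviour that shows the texture matching an image parameter's current index on a UMG Image.
; Its StartBehaviorParam calls the parent, then casts the owner parameter to BP_ImageParameterSimple and caches it.
; It sets the passed Image's brush from the parameter's Images array, matching texture size, and returns false if either cast fails.
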(fn `StartBehaviorParam`
  (params (Object :type "Object Object Reference"))
  (returns (ReturnValue :type Boolean))
  (locals (ImageParam :type "/Game/SettingSystem/BP_ImageParameterSimple1 Object Reference"))
  (bind _imageparam (`local.ImageParam`))
  (`parent.StartBehaviorParam` Object)
  (bind _asbp_image_parameter_simple_1 (cast `/Game/SettingSystem/BP_ImageParameterSimple1` (`self.GetOwnerParameter`))
    (:`then`
      (set `local.ImageParam` _asbp_image_parameter_simple_1)
      (bind _asimage (cast `Image` (`local.Object`))
        (:`then`
          (`Image.SetBrushFromTexture` _asimage (`|GetArrayItem` (`/Game/SettingSystem/BP_ImageParameterSimple1.Images` _imageparam) (`CustomParameterBase.GetCurrentIndex` _imageparam)) true)
          (return true))
        (:`CastFailed`
          _)))
    (:`CastFailed`
      _))
  (return false))