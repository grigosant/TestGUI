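; BP_FloatParameterSimple is a setting-system parameter that holds float variants and can use the selected one as a timer duration.
; ChooseOneOfVariants defers to the parent, while FillStringVariants converts the variants, prints the first converted entry and returns true.
; StartTimer sets an event timer from the variant at the current index, and TimerFinished calls OnTimeIsOver.
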(fn `ChooseOneOfVariants`
  (params (SelectedNumber :type Integer))
  (returns (ReturnValue :type Boolean))
  (bind _returnvalue (`parent.ChooseOneOfVariants` SelectedNumber))
  (return _returnvalue))

(fn `FillStringVariants`
  (returns (ReturnValue :type Boolean))
  (bind _first (`self.VariantsConvert` (`self.Variants`)))
  (`KismetSystemLibrary.PrintString` null (`KismetStringLibrary.Conv_DoubleToString` _first))
  (return true))

(fn `StartTimer`
  (`KismetSystemLibrary.K2_SetTimerDelegate` (`|CreateDelegate` :!event `TimerFinished`) (`|GetArrayItem` (`self.Variants`) (`self.GetCurrentIndex`))))

(fn `TimerFinished`
  (`self.OnTimeIsOver`))