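; Game mode Blueprint in the SettingSystem folder that exercises configurable game rules with debug output.
; On BeginPlay it stores the GameRules parameter struct in SettingsParametersBefore and prints a debug message.
; Disconnected test chains, which never run, set a float rule from a struct with before and after snapshots, print the rule-name count, and select a variant of a named parameter.
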(event `self.ReceiveBeginPlay`
  (`|ExecutionSequence`
    (:`then_0`
      (set `self.SettingsParametersBefore` (`SettingsComponent.GetParametersStruct` (`self.GameRules`)))
      (`KismetSystemLibrary.PrintString` "Hello" true true (struct :`G` 0.66 :`B` 1.0 :`A` 1.0) 15.0))))

(fn `UserConstructionScript`)